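; Audio visualizer actor that analyzes a submix and shows its loudness through mesh height, material glow and a percentage label.
; Each tick it averages magnitudes at chosen frequencies and normalizes against a recorded peak, which a looping timer decays so the range adapts.
; It also copies raw magnitudes to the first Global1 actor, adds a Chartg widget at start, and debug-prints average volume and loudest frequency.
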(event `self.ReceiveBeginPlay`
  ;[1 1 1] beginplay
  (`|ExecutionSequence`
    (:`then_0`
      ;[1 1 1] Initialize dynamic material
      (bind _returnvalue (`KismetMaterialLibrary.CreateDynamicMaterialInstance` (`self.BaseMaterial`)))
      (set `self.MID` _returnvalue)
      (`PrimitiveComponent.SetMaterial` (`self.StaticMesh`) 0 (`self.MID`)))
    (:`then_1`
      ;[1 1 1] decreaseHistoricMaxVolume
      (`KismetSystemLibrary.K2_SetTimerDelegate` (delegate `LowerHistoricMaxRecordedVol`) 0.5 true))
    (:`then_2`
      ;[1 1 1] start analyzing submix
      (`AudioMixerBlueprintLibrary.StartAnalyzingOutput` (`self.SubmixToVisualize`)))
    (:`then_3`
      (bind _returnvalue_2 (`|CreateWidget` "/Game/chartg.chartg_C"))
      (`UserWidget.AddToViewport` _returnvalue_2 0))))

(event `LowerHistoricMaxRecordedVol`
  ;[1 1 1] decreaseHistoricMaxVolume
  (bind _output_get (set `self.MaxRecordedVol` (* (stale _output_get) 0.95))))

(event `self.ReceiveTick`
  (params (DeltaSeconds :type "Float (single-precision)"))
  (bind _cnt (`self.cnt`))
  ;[1 1 1] tick
  (`|ExecutionSequence`
    (:`then_0`
      (bind _outactors (`GameplayStatics.GetAllActorsOfClass` "/Game/global1.global1_C"))
      (bind _magnitudes (`AudioMixerBlueprintLibrary.GetMagnitudeForFrequencies` (`self.FrequenciesToGetAverageVolFrom`) (`self.SubmixToVisualize`)))
      (bind _output (`|GetArrayItem` _outactors))
      (set `/Game/global1.volumes` _magnitudes _output)
      (`KismetArrayLibrary.Array_Set` _outactors 0 _output))
    (:`then_1`
      (`|ExecutionSequence`
        (:`then_0`
          ;[1 1 1] Store latest submix average volume
          (bind _currentaveragevolume (`self.GetAverageSubmixVolumeThisFrame`))
          (bind _output_get (set `self.LatestVolume` _currentaveragevolume))
          (`KismetSystemLibrary.PrintString` (`KismetStringLibrary.Concat_StrStr` (`KismetStringLibrary.Conv_DoubleToString` _output_get) ";;" (`KismetStringLibrary.Conv_IntToString` _cnt)))
          (`/Engine/EditorBlueprintResources/StandardMacros.IncrementInt` _cnt))
        (:`then_1`
          ;[1 1 1] Normalize volume output values to 0-1
          (`self.NormalizeVolume` (`self.LatestVolume`)))
        (:`then_2`
          ;[1 1 1] visualize
          ;;[1 1 1] Scale mesh
          (if (`self.ScaleMeshToAudio`)
            (`self.UpdateMeshScale`)))
        (:`then_3`
          ;;[1 1 1] Update dynamic material emissive strength
          (if (`self.GlowMaterialToAudio`)
            (`self.UpdateMaterialEmissive`)))
        (:`then_4`
          (bind _frequency (`self.GetFrequencyWithLargestVolume`))
          (`KismetSystemLibrary.PrintString` (`KismetStringLibrary.Concat_StrStr` "Freq: " (`KismetStringLibrary.Conv_DoubleToString` (`KismetMathLibrary.BreakVector2D` _frequency)) "," (`KismetStringLibrary.Conv_DoubleToString` (`.Y` (`KismetMathLibrary.BreakVector2D` _frequency))))))
        (:`then_5`
          ;;[1 1 1] update volume % text display
          (if (`self.ShowTextInfo`)
            (`self.UpdateText`)
            (else
              ;;[1 1 1] destroy text preview component
              (`/Engine/EditorBlueprintResources/StandardMacros.DoOnce` false
                (:`Completed`
                  (`ActorComponent.K2_DestroyComponent` (`self.TextRenderVolumePercent`)))))))))))

(fn `GetAverageSubmixVolumeThisFrame`
  (returns (CurrentAverageVolume :type "Float (double-precision)"))
  (locals (AddTogether :type "Float (double-precision)"))
  ;[1 1 1] get latest from submix
  (bind _magnitudes (`AudioMixerBlueprintLibrary.GetMagnitudeForFrequencies` (`self.FrequenciesToGetAverageVolFrom`) (`self.SubmixToVisualize`)))
  ;[1 1 1] add volume for all freqs together
  (for _array_element _magnitudes
    (bind _output_get (set `local.AddTogether` (+ (stale _output_get) _array_element))))
  (return (/ _output_get (`KismetMathLibrary.Conv_IntToDouble` (`KismetArrayLibrary.Array_Length` _magnitudes)))))

(fn `GetFrequencyWithLargestVolume`
  (returns (frequency :type "Vector2D Structure"))
  (locals (baseVolume :type "Vector2D Structure"))
  (bind (_basevolume_x _basevolume_y) (`KismetMathLibrary.BreakVector2D` (`local.baseVolume`)))
  (bind (_basevolume_x_2 _basevolume_y_2) (`KismetMathLibrary.BreakVector2D` (`local.baseVolume`)))
  ;[1 1 1] get latest from submix
  (bind _magnitudes (`AudioMixerBlueprintLibrary.GetMagnitudeForFrequencies` (`self.FrequenciesToGetAverageVolFrom`) (`self.SubmixToVisualize`)))
  (for (_array_element _array_index) _magnitudes
    (if (> _array_element _basevolume_y)
      (set `local.baseVolume` (`KismetMathLibrary.MakeVector2D` (`KismetMathLibrary.Conv_IntToDouble` _array_index) _array_element))))
  (return (`KismetMathLibrary.MakeVector2D` (`|GetArrayItem` (`self.FrequenciesToGetAverageVolFrom`) (`KismetMathLibrary.FTrunc` _basevolume_x_2)) _basevolume_y_2)))

(fn `NormalizeVolume`
  (params (LatestEnvelopeValue :type "Float (double-precision)"))
  (returns (NormalizedVolume :type "Float (double-precision)"))
  (locals (_latestEnvelope :type "Float (double-precision)"))
  ;[1 1 1] Store latest value locally
  (set `local._latestEnvelope` LatestEnvelopeValue)
  (`|ExecutionSequence`
    (:`then_0`
      ;[1 1 1] Store maximum recorded volume
      (if (> (`local._latestEnvelope`) (`self.MaxRecordedVol`))
        (set `self.MaxRecordedVol` (`local._latestEnvelope`))))
    (:`then_1`
      ;[1 1 1] Normalize to range 0-1
      (set `self.NormalizedVolume` (`KismetMathLibrary.FClamp` (`KismetMathLibrary.NormalizeToRange` (`local._latestEnvelope`) 0.0 (`self.MaxRecordedVol`)))))
    (:`then_2`
      ;[1 1 1] Return
      (return (`self.NormalizedVolume`)))))

(fn `UpdateMaterialEmissive`
  (`MaterialInstanceDynamic.SetScalarParameterValue` (`self.MID`) "Emissive Multiplier" (* (`self.NormalizedVolume`) (`self.MaterialEmissiveStrength`))))

(fn `UpdateMeshScale`
  ;[1 1 1] Scale mesh with volume
  (`SceneComponent.SetRelativeScale3D` (`self.StaticMesh`) (`KismetMathLibrary.MakeVector` 1.0 1.0 (+ (* (`self.NormalizedVolume`) (`self.MeshScaleMultiplier`)) 1.0))))

(fn `UpdateText`
  (bind _returnvalue (`KismetSystemLibrary.GetDisplayName` (`self.SubmixToVisualize`)))
  ;[1 1 1] update text content
  (`TextRenderComponent.K2_SetText` (`self.TextRenderVolumePercent`) (`KismetTextLibrary.Conv_StringToText` (`KismetStringLibrary.Concat_StrStr` (`KismetStringLibrary.Concat_StrStr` (select `bool` (== _returnvalue "") :`false` _returnvalue :`true` "Master Submix") " \nVolume") (`KismetStringLibrary.Conv_IntToString` (`KismetMathLibrary.Round` (* (`self.NormalizedVolume`) 100.0))) "%")))
  ;[1 1 1] update text color
  (`TextRenderComponent.SetTextRenderColor` (`self.TextRenderVolumePercent`) (`KismetMathLibrary.Conv_LinearColorToColor` (`KismetMathLibrary.LinearColorLerp` (struct :`R` 0.34375 :`G` 0.34375 :`B` 0.34375 :`A` 1.0) (struct :`R` 0.005208 :`G` 0.005208 :`B` 0.005208 :`A` 1.0) (`self.NormalizedVolume`)) false)))

(fn `UserConstructionScript`
  (`self.UpdateText`))